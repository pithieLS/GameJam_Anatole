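; BP_AFA_ToyPieceConveyor is a conveyor actor that keeps spawning toy pieces while the game is running.
; It caches the AFA game mode on BeginPlay, and its game-started handler kicks off the spawn loop.
; The loop calls SpawnToyPiece, waits SpawnRate through a Delay, then repeats until the game mode reports the game is no longer running.
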(event `self.ReceiveBeginPlay`
  (`parent.ReceiveBeginPlay`)
  (bind _asafa_game_mode (cast `AFA_GameMode` (`GameplayStatics.GetGameMode`)))
  (set `self.As AFA Game Mode` _asafa_game_mode))

(event `self.OnGameStartedHandler`
  (`self.SpawnToyPieceHandler`))

(event `SpawnToyPieceHandler`
  (if (`AFA_GameMode.GetIsGameRunning` (`self.As AFA Game Mode`)) :!label _label
    (`self.SpawnToyPiece`)
    (`KismetSystemLibrary.Delay` (`self.SpawnRate`))
    (goto _label)))

(fn `UserConstructionScript`)