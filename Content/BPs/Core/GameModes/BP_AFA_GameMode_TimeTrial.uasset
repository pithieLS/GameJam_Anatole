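; Time trial game mode that handles the end of a round by presenting the toy box end screen.
; On game end it creates the end screen widget from its own state, switches input to UI only and shows the cursor.
; It then spawns a toy box RT pawn below the world origin, which spawns the verified toys from the order verification counts.
; BeginPlay and Tick defer to the parent; an unconnected branch holds hard-coded test counts.
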(event `self.ReceiveBeginPlay`
  (`parent.ReceiveBeginPlay`))

(event `self.ReceiveTick`
  (params (DeltaSeconds :type "Float (single-precision)"))
  (`parent.ReceiveTick` DeltaSeconds))

(event `self.OnGameEndedHandler`
  (bind _returnvalue (`GameplayStatics.GetPlayerController` 0))
  (bind _returnvalue_2 (`|CreateWidget` "/Game/UI/EndScreens/WBP_AFA_EndScreenToyBoxWidget.WBP_AFA_EndScreenToyBoxWidget_C"))
  (`AFA_EndScreenToyBoxWidget.UpdateWidget` _returnvalue_2 self)
  (`UserWidget.AddToViewport` _returnvalue_2 0)
  (`WidgetBlueprintLibrary.SetInputMode_UIOnlyEx` _returnvalue null)
  (set `PlayerController.bShowMouseCursor` true _returnvalue)
  (bind _returnvalue_3 (`|SpawnActorFromClass` "/Game/BPs/RenderTargetsActor/BP_AFA_ToyBoxRTPawn.BP_AFA_ToyBoxRTPawn_C" (`KismetMathLibrary.MakeTransform` (0.0 0.0 -1000.0)) "Undefined" "MultiplyWithRoot" null null))
  (`AFA_ToyBoxRTActor.SpawnVerifiedToys` _returnvalue_3 (`self.OrderVerificationCount`)))

(fn `UserConstructionScript`)